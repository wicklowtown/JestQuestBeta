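; Floor tile for a runner game whose box overlap tells the RunnerGame mode to extend the floor and add points.
; The overlap also clamps and prints the Jester's walk speed; its multiplier is 1.0, so speed only changes at the limits.
; Construction builds two spawn points per lane, shuffles them and attaches one or two child-actor obstacles.
; GetAttachPoint returns the Arrow's world transform.
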(event OnComponentBeginOverlap(Box)
  (params (OverlappedComponent :type Primitive%20Component%20Object%20Reference) (OtherActor :type Actor%20Object%20Reference) (OtherComp :type Primitive%20Component%20Object%20Reference) (OtherBodyIndex :type Integer) (bFromSweep :type Boolean) (SweepResult :type Hit%20Result%20Structure%20%28by%20ref%29))
  ;[1 1 1] Extend floor
  (bind _asrunner_game (Utilities|Casting|CastToRunnerGame (Game|GetGameMode)))
  (Default|ExtendFloor _asrunner_game)
  ;[1 1 1] Change speed
  (bind _asjester (Utilities|Casting|CastToJester (Game|GetPlayerCharacter 0)))
  (bind _output_get (Variables|/Script/Engine.CharacterMovementComponent|SetMaxWalkSpeed (Variables|/Script/Engine.Character|GetCharacterMovement _asjester) (Math|Float|Clamp(Float) (* (Variables|/Script/Engine.CharacterMovementComponent|GetMaxWalkSpeed (Variables|/Script/Engine.Character|GetCharacterMovement _asjester)) 1.0) 7.5e+02 1.5e+03)))
  (Development|PrintString (Utilities|String|ToString(Float) _output_get))
  ;[1 1 1] Set Current Score
  (bind _asrunner_game_2 (Utilities|Casting|CastToRunnerGame (Game|GetGameMode)))
  (Variables|/Game/Runner/Blueprints/RunnerGame.RunnerGame_C|SetCurrentPoints _asrunner_game_2 (+ (* (Variables|/Game/Runner/Blueprints/RunnerGame.RunnerGame_C|GetPoints%20Multi _asrunner_game_2) 1) (Variables|/Game/Runner/Blueprints/RunnerGame.RunnerGame_C|GetCurrentPoints _asrunner_game_2))))

(event EventBeginPlay)

(event Collision|EventActorBeginOverlap
  (params (OtherActor :type Actor%20Object%20Reference)))

(event EventTick
  (params (DeltaSeconds :type Float%20%28single-precision%29)))

(fn ConstructionScript
  (CallFunction|SetupSpawnPoints)
  (CallFunction|SpawnObstacles))

(fn GetAttachPoint
  (return (Transformation|GetWorldTransform (Variables|Default|GetArrow))))

(fn SetupSpawnPoints
  (for _array_element (Variables|Components|GetLanePositionofTypeFloat)
    (for _index (range 0 1)
      (bind _returnvalue (AddComponent|AddArrowComponent false (Math|Transform|MakeTransform (Math|Vector|MakeVector (* _index 6.5e+02) _array_element 0.0))))
      (Utilities|Array|Add (Variables|Default|GetNewSpawnPoints) (Transformation|GetWorldTransform _returnvalue)))))

(fn SpawnObstacles
  (bind _output_get (LocalVariables|SetRandomSpawnPoints (Variables|Default|GetNewSpawnPoints)))
  (Utilities|Array|Shuffle _output_get)
  (for _index (range 0 (Math|Random|RandomIntegerinRange 0 1))
    (switch int (Math|Random|RandomIntegerinRange 0 1)
      (:0
        (AddComponent|AddChildActorComponent false (Math|Transform|MakeRelativeTransform (Utilities|Array|Get(acopy) (LocalVariables|GetRandomSpawnPoints) _index) (Transformation|GetActorTransform))))
      (:1
        (AddComponent|AddChildActorComponent false (Math|Transform|MakeRelativeTransform (Utilities|Array|Get(acopy) (LocalVariables|GetRandomSpawnPoints) _index) (Transformation|GetActorTransform)))))))